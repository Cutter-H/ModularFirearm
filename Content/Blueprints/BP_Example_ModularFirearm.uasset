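; Example modular firearm Blueprint that plays first-person montages on the demo character wielding it.
; BeginPlay disables all collision responses on its static mesh components and binds handlers to the firearm's firing and reload montage events.
; Both handlers cast the instigator to BP_DemoCharacter and play the rifle shoot montage on its first-person mesh, so reload reuses the shoot animation.
; Tick prints the current ammo count for debugging.
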(event `self.ReceiveBeginPlay`
  (for _array_element (`self.K2_GetComponentsByClass` "/Script/Engine.StaticMeshComponent")
    (`PrimitiveComponent.SetCollisionResponseToAllChannels` _array_element "ECR_Ignore"))
  (add `self.OnFiringMontagePlay` (delegate `OnFireMontage`))
  (add `self.OnReloadMontagePlay` (delegate `OnReloadMontage`)))

(event `OnFireMontage` :!signature `self.OnFiringMontagePlay`
  (params (montage :type "AnimMontage Object Reference"))
  (bind _asbp_demo_character (cast `/ModularFirearm/Blueprints/BP_DemoCharacter` (`self.GetInstigator`)))
  (`|PlayMontage` (`/ModularFirearm/Blueprints/BP_DemoCharacter.FirstPersonMesh` _asbp_demo_character) "/ModularFirearm/Demo/EpicContent/FirstPersonArms/Animations/FP_Rifle_Shoot_Montage.FP_Rifle_Shoot_Montage"))

(event `OnReloadMontage` :!signature `self.OnReloadMontagePlay`
  (params (montage :type "AnimMontage Object Reference"))
  (bind _asbp_demo_character (cast `/ModularFirearm/Blueprints/BP_DemoCharacter` (`self.GetInstigator`)))
  (`|PlayMontage` (`/ModularFirearm/Blueprints/BP_DemoCharacter.FirstPersonMesh` _asbp_demo_character) "/ModularFirearm/Demo/EpicContent/FirstPersonArms/Animations/FP_Rifle_Shoot_Montage.FP_Rifle_Shoot_Montage"))

(event `self.ReceiveTick`
  (params (DeltaSeconds :type "Float (single-precision)"))
  (`KismetSystemLibrary.PrintString` (`KismetStringLibrary.Concat_StrStr` "Current Ammo: " (`KismetStringLibrary.Conv_IntToString` (`self.GetCurrentAmmo`))) true true (struct :`G` 0.66 :`B` 1.0 :`A` 1.0) 0.0))

(fn `UserConstructionScript`)